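; Fire actor with a particle system that can grow in size over time, plus a Box component whose overlap event is empty.
; The makeBigger event adds a uniform step to the particle's world scale and re-arms a short one-shot timer on itself until all three axis thresholds are met.
; Nothing in this Blueprint starts the growth, and a node that hides the particles is left unconnected.
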(event `self.Box.OnComponentBeginOverlap`
  (params (OverlappedComponent :type "PrimitiveComponent Object Reference") (OtherActor :type "Actor Object Reference") (OtherComp :type "PrimitiveComponent Object Reference") (OtherBodyIndex :type Integer) (bFromSweep :type Boolean) (SweepResult :type "HitResult Structure (by ref)")))

(event `makeBigger`
  (bind _particlesystemcomponent (`self.ParticleSystemComponent`))
  (bind (_returnvalue_x _returnvalue_y _returnvalue_z) (`KismetMathLibrary.BreakVector` (`SceneComponent.K2_GetComponentScale` _particlesystemcomponent)))
  (`SceneComponent.SetWorldScale3D` _particlesystemcomponent (+ (`SceneComponent.K2_GetComponentScale` _particlesystemcomponent) (0.1 0.1 0.1)))
  (if (not (and (>= _returnvalue_x 2.0) (> _returnvalue_y 2.0) (>= _returnvalue_z 10.0)))
    (`KismetSystemLibrary.K2_SetTimerDelegate` (delegate `makeBigger`) 0.1)))

(fn `UserConstructionScript`)