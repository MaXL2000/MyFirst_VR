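; BP_Test2 is a physics actor that motion controllers can pick up and drop, with a ring that breaks away on overlap.
; Pickup disables mesh simulation and attaches the root to the given component; Drop restores physics and detaches.
; The first Box overlap destroys the PhysicsConstraint and replaces the Ring component with a spawned BP_Ring at its transform.
; StartShoot sets CanDestroy, which the overlap ignores; material-swap and attach nodes are unwired.
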(event `/Game/VirtualRealityBP/Blueprints/PickupActorInterface.Pickup`
  (params (AttachTo :type "SceneComponent Object Reference"))
  (`PrimitiveComponent.SetSimulatePhysics` (`self.StaticMeshComponent`) false)
  (`SceneComponent.K2_AttachToComponent` (`self.K2_GetRootComponent`) AttachTo "None" "KeepWorld" "KeepWorld" "KeepWorld" false))

(event `/Game/VirtualRealityBP/Blueprints/PickupActorInterface.Drop`
  (`PrimitiveComponent.SetSimulatePhysics` (`self.StaticMeshComponent`) true)
  (`self.K2_DetachFromActor` "KeepWorld" "KeepWorld" "KeepWorld"))

(event `self.Box.OnComponentBeginOverlap`
  (params (OverlappedComponent :type "PrimitiveComponent Object Reference") (OtherActor :type "Actor Object Reference") (OtherComp :type "PrimitiveComponent Object Reference") (OtherBodyIndex :type Integer) (bFromSweep :type Boolean) (SweepResult :type "HitResult Structure (by ref)"))
  (if (not (`self.Destroyed`))
    (`ActorComponent.K2_DestroyComponent` (`self.PhysicsConstraint`))
    (set `self.Destroyed` true)
    (bind _returnvalue (`|SpawnActorFromClass` "/Game/Blueprints/BP_Ring.BP_Ring_C" (`SceneComponent.K2_GetComponentToWorld` (`self.Ring`)) "Undefined" "OverrideRootScale" null null))
    (`ActorComponent.K2_DestroyComponent` (`self.Ring`))))

(event `self.Box.OnComponentEndOverlap`
  (params (OverlappedComponent :type "PrimitiveComponent Object Reference") (OtherActor :type "Actor Object Reference") (OtherComp :type "PrimitiveComponent Object Reference") (OtherBodyIndex :type Integer)))

(fn `start_shoot`
  (params (Shoot :type Boolean))
  (returns (NewParam1 :type Boolean))
  (set `self.Can Destroy` Shoot)
  (return false))

(fn `UserConstructionScript`)