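; BP_AK47 is a VR rifle that a motion controller can pick up and drop, and that destroys pickup cubes it aims at.
; Pickup and Drop toggle mesh physics and attach or detach the actor.
; Every tick, a visible debug line trace runs forward from the mesh.
; While CanDestroy, set through StartShoot, is true, any BP_PickupCube or BP_PickupCube1 hit is destroyed.
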(event `/Game/VirtualRealityBP/Blueprints/PickupActorInterface.Pickup`
  (params (AttachTo :type "SceneComponent Object Reference"))
  (`PrimitiveComponent.SetSimulatePhysics` (`self.StaticMeshComponent`) false)
  (`SceneComponent.K2_AttachToComponent` (`self.K2_GetRootComponent`) AttachTo "None" "KeepWorld" "KeepWorld" "KeepWorld" false))

(event `/Game/VirtualRealityBP/Blueprints/PickupActorInterface.Drop`
  (`PrimitiveComponent.SetSimulatePhysics` (`self.StaticMeshComponent`) true)
  (`self.K2_DetachFromActor` "KeepWorld" "KeepWorld" "KeepWorld"))

(event `self.Box.OnComponentBeginOverlap`
  (params (OverlappedComponent :type "PrimitiveComponent Object Reference") (OtherActor :type "Actor Object Reference") (OtherComp :type "PrimitiveComponent Object Reference") (OtherBodyIndex :type Integer) (bFromSweep :type Boolean) (SweepResult :type "HitResult Structure (by ref)")))

(event `self.ReceiveTick`
  (params (DeltaSeconds :type "Float (single-precision)"))
  (bind _staticmeshcomponent (`self.StaticMeshComponent`))
  (bind _returnvalue (`SceneComponent.K2_GetComponentLocation` _staticmeshcomponent))
  (bind _outhit (`KismetSystemLibrary.LineTraceSingle` :`Start` _returnvalue :`End` (+ _returnvalue (* (`KismetMathLibrary.GetForwardVector` (`SceneComponent.K2_GetComponentRotation` _staticmeshcomponent)) 2000.0)) :`TraceChannel` "TraceTypeQuery1" :`DrawDebugType` "ForOneFrame" :`TraceColor` (struct :`R` 1.0 :`G` 0.060103 :`B` 0.147777 :`A` 1.0)))
  (`|ExecutionSequence`
    (:`then_0`
      (bind (_bblockinghit _binitialoverlap _time _distance _location _impactpoint _normal _impactnormal _physmat _hitactor) (`GameplayStatics.BreakHitResult` _outhit))
      (bind _asbp_pickup_cube (cast `/Game/VirtualRealityBP/Blueprints/BP_PickupCube` _hitactor))
      (`/Engine/EditorBlueprintResources/StandardMacros.IsValid` _asbp_pickup_cube
        (:`Is Valid`
          (if (`self.Can Destroy`)
            (`self.K2_DestroyActor` _asbp_pickup_cube)))))
    (:`then_1`
      (bind _asbp_pickup_cube_1 (cast `/Game/VirtualRealityBP/Blueprints/BP_PickupCube1` _hitactor))
      (`/Engine/EditorBlueprintResources/StandardMacros.IsValid` _asbp_pickup_cube_1
        (:`Is Valid`
          (if (`self.Can Destroy`)
            (`self.K2_DestroyActor` _asbp_pickup_cube_1)))))))

(fn `start_shoot`
  (params (Shoot :type Boolean))
  (returns (NewParam1 :type Boolean))
  (set `self.Can Destroy` Shoot)
  (return false))

(fn `UserConstructionScript`)